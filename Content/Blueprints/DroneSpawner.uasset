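; Drone spawner actor that keeps populating the level with BP_DronePawn until 40 exist.
; On BeginPlay it caches all PatrolPoint actors, spawns a drone, then loops on a three-second delay, spawning again whenever CanSpawn finds room under the cap.
; Each drone spawns at a random patrol point and receives that same point as GoalActor.
; The random index range excludes the last cached point.
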(event EventBeginPlay
  (bind _outactors (Actor|GetAllActorsOfClass "/Game/Blueprints/Drone/PatrolPoint.PatrolPoint_C"))
  (bind _output_get (Variables|Default|SetPatrolPoints _outactors))
  (Variables|Default|SetMaxLength (Utilities|Array|Length _output_get))
  (Development|PrintString (Utilities|String|ToString(Integer) (Utilities|Array|Length _output_get)))
  (CallFunction|SpawnDrone :!label _label)
  (Utilities|FlowControl|Delay 3.0 :!label _label_2)
  (bind _canspawn (CallFunction|CanSpawn))
  (if _canspawn
    (goto _label)
    (else
      (goto _label_2))))

(event Collision|EventActorBeginOverlap
  (params (OtherActor :type Actor%20Object%20Reference)))

(event EventTick
  (params (DeltaSeconds :type Float%20%28single-precision%29)))

(fn ConstructionScript)

(fn SpawnDrone
  (bind _aspatrol_point (CallFunction|GetRandomPatrolPoint))
  (bind _returnvalue (Game|SpawnActorfromClass "/Game/Blueprints/Drone/BP_DronePawn.BP_DronePawn_C" (Math|Transform|MakeTransform (Transformation|GetActorLocation _aspatrol_point) "0, 0, 0" "1.000000,1.000000,1.000000") "Undefined" 0 0))
  (Utilities|IsValid _returnvalue
    (:Is%20Valid
      (Variables|/Game/Blueprints/Drone/BP_DronePawn.BP_DronePawn_C|SetGoal%20Actor _returnvalue _aspatrol_point))))

(fn GetRandomPatrolPoint
  (bind _aspatrol_point (Utilities|Casting|CastToPatrolPoint (Utilities|Array|Get(acopy) (Variables|Default|GetPatrolPoints) (Math|Random|RandomInteger (- (Variables|Default|GetMaxLength) 1)))))
  (return _aspatrol_point))

(fn CanSpawn
  (bind _outactors (Actor|GetAllActorsOfClass "/Game/Blueprints/Drone/BP_DronePawn.BP_DronePawn_C"))
  (return (< (Utilities|Array|Length _outactors) 40)))